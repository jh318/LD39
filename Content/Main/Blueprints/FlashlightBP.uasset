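; Player flashlight actor that follows the player character, turns toward the cursor and toggles its light on left click.
; Tick updates position and rotation, and a shared macro checks whether the light is visible.
; A forward sphere trace flags hits on Enemy-tagged actors, alongside intensity drain and a FlashlightHitEnemy call.
; The construction script caches the first BasicEnemy found; debug prints and trace drawing remain.
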(event `InputAction|LeftClick`
  (params (Key :type "Key Structure" :default "AnyKey"))
  (:`Pressed`
    (`self.ToggleFlashlight`)
    (if (`SceneComponent.IsVisible` (`self.Flashlight`))
      (`self.SphereCastForEnemies` :!label _label)
      (`self.LoseIntensityWhileOn`)
      (`self.FlashlightHitEnemy`))))

(event `self.ReceiveTick`
  (params (DeltaSeconds :type "Float (single-precision)"))
  (`self.SetToPlayerLocation`)
  (`self.RotateToMouse`)
  (if (`SceneComponent.IsVisible` (`self.Flashlight`))
    (goto _label)))

(fn `LoseIntensityWhileOn`
  (if (> (`LightComponentBase.Intensity` (`self.Flashlight`)) 0.0)
    (`LightComponent.SetIntensity` (`self.Flashlight`) (- (`LightComponentBase.Intensity` (`self.Flashlight`)) 10.0))))

(fn `RotateToMouse`
  (`SceneComponent.K2_SetRelativeRotation` (`self.FlashlightSprite`) (`KismetMathLibrary.MakeRotator` (.roll (`KismetMathLibrary.FindLookAtRotation` (`SceneComponent.K2_GetComponentLocation` (`self.FlashlightSprite`)) (`.Location` (`GameplayStatics.BreakHitResult` (`PlayerController.GetHitResultUnderCursorByChannel` (`GameplayStatics.GetPlayerController` 0) "TraceTypeQuery1" true))))) (.pitch (`KismetMathLibrary.FindLookAtRotation` (`SceneComponent.K2_GetComponentLocation` (`self.FlashlightSprite`)) (`.Location` (`GameplayStatics.BreakHitResult` (`PlayerController.GetHitResultUnderCursorByChannel` (`GameplayStatics.GetPlayerController` 0) "TraceTypeQuery1" true))))) (.yaw (`KismetMathLibrary.FindLookAtRotation` (`SceneComponent.K2_GetComponentLocation` (`self.FlashlightSprite`)) (`.Location` (`GameplayStatics.BreakHitResult` (`PlayerController.GetHitResultUnderCursorByChannel` (`GameplayStatics.GetPlayerController` 0) "TraceTypeQuery1" true)))))) false false))

(fn `SetToPlayerLocation`
  (`SceneComponent.K2_SetWorldLocation` (`self.DefaultSceneRoot`) (`self.K2_GetActorLocation` (`GameplayStatics.GetPlayerCharacter` 0)) false false))

(fn `SphereCastForEnemies`
  (bind _flashlightsprite (`self.FlashlightSprite`))
  (bind _returnvalue (`SceneComponent.K2_GetComponentLocation` _flashlightsprite))
  (bind _outhit (`KismetSystemLibrary.SphereTraceSingle` :`Start` _returnvalue :`End` (+ _returnvalue (* (`KismetMathLibrary.GetForwardVector` (`SceneComponent.K2_GetComponentRotation` _flashlightsprite)) 1000.0)) :`Radius` 75.0 :`TraceChannel` "TraceTypeQuery1" :`DrawDebugType` "ForOneFrame"))
  (if (`self.ActorHasTag` (`.HitActor` (`GameplayStatics.BreakHitResult` _outhit)) "Enemy")
    (`KismetSystemLibrary.PrintString` "Enemy Detected")
    (set `self.flashlightIsColliding` true)
    (else
      (`KismetSystemLibrary.PrintString` "Nothing"))))

(fn `ToggleFlashlight`
  (if (`SceneComponent.bVisible` (`self.Flashlight`))
    (`SceneComponent.SetVisibility` (`self.Flashlight`) false false)
    (else
      (`SceneComponent.SetVisibility` (`self.Flashlight`) true false))))

(fn `UserConstructionScript`
  (bind _outactors (`GameplayStatics.GetAllActorsOfClass` "/Game/Main/Blueprints/BasicEnemy.BasicEnemy_C"))
  (bind _asbasic_enemy (cast `/Game/Main/Blueprints/BasicEnemy` (`|GetArrayItem` _outactors)))
  (set `self.basicEnemyReference` _asbasic_enemy))