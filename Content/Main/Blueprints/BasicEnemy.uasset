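; BasicEnemy is a side-facing sprite enemy that chases the player and destroys it on touching its collider.
; A detection radius toggles the chase, and Tick moves the enemy by a fraction of the remaining distance, so it slows as it closes in.
; It yaws to face the player, and a Frozen flag pauses movement until a delay clears it.
; The construction script caches a flashlight reference, but its hit binding is disconnected.
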(event `IsHit_Event`)

(event `self.ReceiveBeginPlay`
  (set `self.speedGame` (`self.speedStart`)))

(event `self.DetectionRadius.OnComponentEndOverlap`
  (params (OverlappedComponent :type "PrimitiveComponent Object Reference") (OtherActor :type "Actor Object Reference") (OtherComp :type "PrimitiveComponent Object Reference") (OtherBodyIndex :type Integer))
  (if (`self.ActorHasTag` OtherActor "Player")
    (set `self.playerInRange` false)))

(event `self.DetectionRadius.OnComponentBeginOverlap`
  (params (OverlappedComponent :type "PrimitiveComponent Object Reference") (OtherActor :type "Actor Object Reference") (OtherComp :type "PrimitiveComponent Object Reference") (OtherBodyIndex :type Integer) (bFromSweep :type Boolean) (SweepResult :type "HitResult Structure (by ref)"))
  (if (`self.ActorHasTag` OtherActor "Player")
    (set `self.playerInRange` true)))

(event `self.ReceiveTick`
  (params (DeltaSeconds :type "Float (single-precision)"))
  (`|ExecutionSequence`
    (:`then_0`
      (if (`self.playerInRange`)
        (if (`self.frozen`)
          (`KismetSystemLibrary.Delay` (`self.resetMovementSeconds`))
          (set `self.frozen` false)
          (else
            (`self.MoveTowardsPlayer` DeltaSeconds)))))
    (:`then_1`
      (`self.RotateEnemySprite`))))

(event `self.EnemyCollider.OnComponentBeginOverlap`
  (params (OverlappedComponent :type "PrimitiveComponent Object Reference") (OtherActor :type "Actor Object Reference") (OtherComp :type "PrimitiveComponent Object Reference") (OtherBodyIndex :type Integer) (bFromSweep :type Boolean) (SweepResult :type "HitResult Structure (by ref)"))
  (if (`self.ActorHasTag` OtherActor "Player")
    (`self.K2_DestroyActor` OtherActor)
    (`self.PlayerDestroyed`)))

(fn `MoveTowardsPlayer`
  (params (B :type "Float (double-precision)"))
  (bind _returnvalue (`self.K2_GetActorLocation`))
  (`self.K2_SetActorLocation` (+ _returnvalue (* (* (- (`self.K2_GetActorLocation` (`GameplayStatics.GetPlayerPawn` 0)) _returnvalue) B) (`self.speedGame`)))))

(fn `RotateEnemySprite`
  (bind _returnvalue_x (`KismetMathLibrary.BreakVector` (`SceneComponent.K2_GetComponentLocation` (`self.EnemySprite`))))
  (bind _returnvalue_x_2 (`KismetMathLibrary.BreakVector` (`SceneComponent.K2_GetComponentLocation` (`Character.CapsuleComponent` (`GameplayStatics.GetPlayerCharacter` 0)))))
  (`/Engine/EditorBlueprintResources/StandardMacros.CompareFloat` _returnvalue_x _returnvalue_x_2
    (:`>`
      (`self.K2_SetActorRotation` (`ActorComponent.GetOwner` (`self.EnemyCollider`)) (`KismetMathLibrary.MakeRotator` 0.0 0.0 180.0) false))
    (:`<`
      (`self.K2_SetActorRotation` (`ActorComponent.GetOwner` (`self.EnemyCollider`)) (`KismetMathLibrary.MakeRotator` 0.0 0.0 0.0) false))))

(fn `UserConstructionScript`
  (bind _outactors (`GameplayStatics.GetAllActorsOfClass` "/Game/Main/Blueprints/FlashlightBP.FlashlightBP_C"))
  (bind _asflashlight_bp (cast `/Game/Main/Blueprints/FlashlightBP` (`|GetArrayItem` _outactors)))
  (set `self.flashlightReference` _asflashlight_bp))